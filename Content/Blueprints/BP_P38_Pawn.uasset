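; BP_P38_Pawn is a P-38 airplane pawn that animates its twin propellers.
; Each Tick rolls the Left and Right components in opposite directions at PropellerRotateSpeed, scaled by world delta seconds for frame-rate independence.
; The Roll axis input only prints its value, and the airplane movement nodes are unconnected, so this graph does not move the pawn.
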(event EventBeginPlay)

(event Collision|EventActorBeginOverlap
  (params (OtherActor :type Actor%20Object%20Reference)))

(event EventTick
  (params (DeltaSeconds :type Float%20%28single-precision%29))
  (Utilities|FlowControl|Sequence
    (:then_0
      ;[1 1 1] 왼쪽 프로펠러 회전
      (Transformation|AddLocalRotation (Variables|Default|GetLeft) (Math|Rotator|MakeRotator (* (Variables|Default|GetPropellerRotateSpeed) (Utilities|Time|GetWorldDeltaSeconds)) 0.0 0.0) false false))
    (:then_1
      ;[1 1 1] 오른쪽 프로펠러 회전
      (Transformation|AddLocalRotation (Variables|Default|GetRight) (Math|Rotator|MakeRotator (* (Variables|Default|GetPropellerRotateSpeed) (Utilities|Time|GetWorldDeltaSeconds) -1.0) 0.0 0.0) false false))))

(event Input|AxisEvents|InputAxisRoll
  (params (AxisValue :type Float%20%28single-precision%29))
  (Development|PrintString (Utilities|String|ToString(Float) AxisValue)))

(fn ConstructionScript)