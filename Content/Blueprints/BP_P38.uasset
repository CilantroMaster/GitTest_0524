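; BP_P38 is a P-38 airplane Blueprint with animated twin propellers and placeholder flight logic.
; Each Tick rolls the Left and Right propeller components in opposite directions by PropellerRotateSpeed scaled by delta time.
; Tick also calls a world offset for movement, but its X value is multiplied from zero, so the plane stays still.
; The Roll input axis only prints its value and does not yet steer the plane.
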(event EventBeginPlay)

(event Collision|EventActorBeginOverlap
  (params (OtherActor :type Actor%20Object%20Reference)))

(event EventTick
  (params (DeltaSeconds :type Float%20%28single-precision%29))
  ;[1 1 1] 왼쪽 프로펠러 회전
  (Transformation|AddLocalRotation (Variables|Default|GetLeft) (Math|Rotator|MakeRotator (* (Variables|Default|GetPropellerRotateSpeed) (Utilities|Time|GetWorldDeltaSeconds)) 0.0 0.0) false false)
  ;[1 1 1] 오른쪽 프로펠러 회전
  (Transformation|AddLocalRotation (Variables|Default|GetRight) (Math|Rotator|MakeRotator (* (Variables|Default|GetPropellerRotateSpeed) (Utilities|Time|GetWorldDeltaSeconds) -1.0) 0.0 0.0) false false)
  ;[1 1 1] 비행기 이동
  (Transformation|AddActorWorldOffset self (Math|Vector|MakeVector (* 0.0 (Utilities|Time|GetWorldDeltaSeconds)) 0.0 0.0)))

(event Input|AxisEvents|InputAxisRoll
  (params (AxisValue :type Float%20%28single-precision%29))
  (Development|PrintString (Utilities|String|ToString(Float) AxisValue)))

(fn ConstructionScript)